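; Player hero character that uses the Gameplay Ability System for a three-step normal attack combo, dash, laser, fireball and health regen.
; NormalAttack activates the ability for the current combo count, while DeterminCombo advances that count and sets damage level and montage.
; Other skills reset the combo before activating, and hostile overlaps on the attack collider send a damage gameplay event to self.
; Health updates drive the battle GameMode's HP bar; mana changes are unhandled.
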(event OnComponentBeginOverlap(NormalAttackCol)
  (params (OverlappedComponent :type Primitive%20Component%20Object%20Reference) (OtherActor :type Actor%20Object%20Reference) (OtherComp :type Primitive%20Component%20Object%20Reference) (OtherBodyIndex :type Integer) (bFromSweep :type Boolean) (SweepResult :type Hit%20Result%20Structure%20%28by%20ref%29))
  (if (!= self OtherActor)
    (bind _ascharacter_base (Utilities|Casting|CastToCharacterBase OtherActor))
    (bind _returnvalue (Class|CharacterBase|IsOtherHostile _ascharacter_base self))
    (if _returnvalue
      (Ability|SendGameplayEventtoActor self "(TagName=\"skill.NormalAttack.dealDamage\")" (Utilities|Struct|MakeGameplayEventData "" 0 OtherActor)))))

(event Custom|NormalAttack
  ;[1 1 1] Skill Event
  (switch int (Variables|Default|GetAttackComboCount)
    (:1
      (Abilities|TryActivateAbilitybyClass (Variables|Default|GetAbilitySystemComp) "/Game/Blueprints/Character/Ability/NormalAttack/GA_Hero_NormalAttack_1.GA_Hero_NormalAttack_1_C" true))
    (:2
      (Abilities|TryActivateAbilitybyClass (Variables|Default|GetAbilitySystemComp) "/Game/Blueprints/Character/Ability/NormalAttack/GA_Hero_NormalAttack_2.GA_Hero_NormalAttack_2_C" true))
    (:3
      (Abilities|TryActivateAbilitybyClass (Variables|Default|GetAbilitySystemComp) "/Game/Blueprints/Character/Ability/NormalAttack/GA_Hero_NormalAttack_3.GA_Hero_NormalAttack_3_C" true))))

(event Custom|TryHealthRegen
  ;[1 1 1] Skill Event
  (CallFunction|ResetComboCount)
  (Abilities|TryActivateAbilitybyClass (Variables|Default|GetAbilitySystemComp) "/Game/Blueprints/Character/Ability/HealthRegen/GA_HealthRegen.GA_HealthRegen_C" true))

(event Custom|TryDash
  ;[1 1 1] Skill Event
  (CallFunction|ResetComboCount)
  (Abilities|TryActivateAbilitybyClass (Variables|Default|GetAbilitySystemComp) "/Game/Blueprints/Character/Ability/Dash/GA_Dash.GA_Dash_C" true))

(event Custom|ResetAttackComboCount
  (Variables|Default|SetAttackComboCount 1))

(event Custom|TryLazer
  ;[1 1 1] Skill Event
  (CallFunction|ResetComboCount)
  (Abilities|TryActivateAbilitybyClass (Variables|Default|GetAbilitySystemComp) "/Game/Blueprints/Character/Ability/Lazer/GA_Lazer.GA_Lazer_C" true))

(event Custom|UpdatePlayerHUD
  (Default|UpdateHPBar (.AsBP%20Game%20Mode%20Battle (Utilities|Casting|CastToBP_GameModeBattle (Game|GetGameMode))) (/ (.CurrentValue (Utilities|Struct|BreakGameplayAttributeData (Variables|/Script/ProjectARPG.AttributeSetBase|GetHealth (Variables|Default|GetAttributeSetBaseComp)))) (.CurrentValue (Utilities|Struct|BreakGameplayAttributeData (Variables|/Script/ProjectARPG.AttributeSetBase|GetMaxHealth (Variables|Default|GetAttributeSetBaseComp)))))))

(event Custom|TryFireBall
  ;[1 1 1] Skill Event
  (CallFunction|ResetComboCount)
  (Abilities|TryActivateAbilitybyClass (Variables|Default|GetAbilitySystemComp) "/Game/Blueprints/Character/Ability/FireBall/GA_FireBall.GA_FireBall_C" true))

(event EventBeginPlay
  (|CallParentFunction)
  (Class|CharacterBase|AquireAbilities (Variables|Default|GetInitialAbilities))
  (Class|AttributeSetBase|UpdateActorAttr (Variables|Default|GetAttributeSetBaseComp))
  (CallFunction|UpdatePlayerHUD))

(event Collision|EventActorBeginOverlap
  (params (OtherActor :type Actor%20Object%20Reference))
  (|CallParentFunction OtherActor) ; This node is disabled and will not be called.\nDrag off pins to build functionality.
)

(event EventTick
  (params (DeltaSeconds :type Float%20%28single-precision%29))
  (|CallParentFunction DeltaSeconds) ; This node is disabled and will not be called.\nDrag off pins to build functionality.
)

(event EventOnHealthChanged
  (params (Health :type Float%20%28single-precision%29) (MaxHealth :type Float%20%28single-precision%29))
  (Default|UpdateHPBar (.AsBP%20Game%20Mode%20Battle (Utilities|Casting|CastToBP_GameModeBattle (Game|GetGameMode))) (/ Health MaxHealth)))

(event EventOnManaChanged
  (params (Mana :type Float%20%28single-precision%29) (MaxMana :type Float%20%28single-precision%29)))

(fn ConstructionScript
  (|CallParentFunction))

(fn DeterminCombo
  (switch int (Variables|Default|GetAttackComboCount)
    (:1
      (Variables|Default|SetAttackComboCount 2)
      (bind _output_get (Variables|Default|SetComboDamageLevel 1))
      (Variables|Default|SetNormalAttackMontage "/Game/Blueprints/Character/Animation/AM_NormalAttack_01.AM_NormalAttack_01")
      (return _output_get))
    (:2
      (Variables|Default|SetAttackComboCount 3)
      (bind _output_get_2 (Variables|Default|SetComboDamageLevel 2))
      (Variables|Default|SetNormalAttackMontage "/Game/Blueprints/Character/Animation/AM_NormalAttack_02.AM_NormalAttack_02")
      (return _output_get_2))
    (:3
      (Variables|Default|SetAttackComboCount 1)
      (bind _output_get_3 (Variables|Default|SetComboDamageLevel 3))
      (Variables|Default|SetNormalAttackMontage "/Game/Blueprints/Character/Animation/AM_NormalAttack_03.AM_NormalAttack_03")
      (return _output_get_3))))