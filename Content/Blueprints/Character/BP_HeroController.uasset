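; Hero player controller that creates the primary UI on begin play and steers the controlled pawn from GoUp and GoRight axis input.
; Each axis adds movement input along fixed world X or Y, scaled by Speed, with Force enabled only for GoUp.
; A second pair of handlers for the same axes sets control rotation from a vector built from axis values, once its length passes a small dead zone.
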(event EventBeginPlay
  (bind _returnvalue (UserInterface|CreateWidget "/Game/UI/WBP_PrimaryUI.WBP_PrimaryUI_C"))
  (bind _output_get (Variables|Default|SetPrimaryUI _returnvalue))
  (UserInterface|Viewport|AddtoViewport _output_get 0))

(event EventTick
  (params (DeltaSeconds :type Float%20%28single-precision%29)))

(event Input|ActionEvents|InputActionDash
  (params (Key :type Key%20Structure :default "None")))

(event Input|ActionEvents|InputActionHealthRegen
  (params (Key :type Key%20Structure :default "None")))

(event Input|AxisEvents|InputAxisGoUp
  (params (AxisValue :type Float%20%28single-precision%29))
  (Pawn|Input|AddMovementInput (Pawn|GetControlledPawn) "1.000000, 0, 0" (* AxisValue (Variables|Default|GetSpeed)) true))

(event Input|AxisEvents|InputAxisGoRight
  (params (AxisValue :type Float%20%28single-precision%29))
  (Pawn|Input|AddMovementInput (Pawn|GetControlledPawn) "0.000000,1.000000, 0" (* AxisValue (Variables|Default|GetSpeed)) false))

(event Input|AxisEvents|InputAxisGoUp
  (params (AxisValue :type Float%20%28single-precision%29))
  (if (> (Math|Vector|VectorLength (Math|Vector|MakeVector AxisValue (stale Input|AxisEvents|InputAxisGoRight AxisValue) 0.0)) 0.1)
    (Pawn|SetControlRotation self (Math|Conversions|RotationFromXVector (Math|Vector|MakeVector AxisValue (stale Input|AxisEvents|InputAxisGoRight AxisValue) 0.0)))))

(event Input|AxisEvents|InputAxisGoRight
  (params (AxisValue :type Float%20%28single-precision%29))
  (if (> (Math|Vector|VectorLength (Math|Vector|MakeVector (stale Input|AxisEvents|InputAxisGoUp AxisValue) AxisValue 0.0)) 0.1)
    (Pawn|SetControlRotation self (Math|Conversions|RotationFromXVector (Math|Vector|MakeVector (stale Input|AxisEvents|InputAxisGoUp AxisValue) AxisValue 0.0)))))

(fn ConstructionScript)