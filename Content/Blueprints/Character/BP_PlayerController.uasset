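; Player controller for a twin-stick action game that creates the primary HUD and routes input to the hero.
; Movement, attacks, dash, heal and fireball are gated by the player state's BattleAble flag.
; The aim stick takes over facing from movement, switches to aim speed and enables shooting.
; Menu navigation and weapon-wheel angles go to BP_GameModeBattle, with the wheel suspending combat; OpenMenu quits the game outright.
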(event Custom|SetInterateObjEnable
  (params (Enable :type Boolean)))

(event EventBeginPlay
  (bind _returnvalue (UserInterface|CreateWidget "/Game/UI/WBP_PrimaryUI.WBP_PrimaryUI_C"))
  (bind _output_get (Variables|Default|SetPrimaryUI _returnvalue))
  (UserInterface|Viewport|AddtoViewport _output_get 0)
  (Variables|Default|SetMyPlayerState (.AsBP%20My%20Player%20State (Utilities|Casting|CastToBP_MyPlayerState (Variables|Default|GetPlayerState))))
  (bind _asbp_hero_unit (Utilities|Casting|CastToBP_HeroUnit (Pawn|GetControlledPawn)))
  (Variables|Default|SetHero _asbp_hero_unit))

(event EventTick
  (params (DeltaSeconds :type Float%20%28single-precision%29)))

(event EventAddAbilitytoUI
  (params (AbilityInfo :type Gameplay%20Ability%20Info%20Structure))
  (Default|AddAbilitytoSlots (Variables|Default|GetPrimaryUI) AbilityInfo))

(event Input|ActionEvents|InputActionDash
  (params (Key :type Key%20Structure :default "None"))
  (:Pressed
    (if (Variables|/Game/Blueprints/BP_MyPlayerState.BP_MyPlayerState_C|GetBattleAble (Variables|Default|GetMyPlayerState))
      (Default|TryDash (Variables|Default|GetHero)))))

(event Input|ActionEvents|InputActionHealthRegen
  (params (Key :type Key%20Structure :default "None"))
  (:Pressed
    (if (Variables|/Game/Blueprints/BP_MyPlayerState.BP_MyPlayerState_C|GetBattleAble (Variables|Default|GetMyPlayerState))
      (Default|TryHealthRegen (Variables|Default|GetHero)))))

(event Input|ActionEvents|InputActionUI_Left
  (params (Key :type Key%20Structure :default "None"))
  ;[1 1 1] UI
  (:Pressed
    (bind _asbp_game_mode_battle (Utilities|Casting|CastToBP_GameModeBattle (Game|GetGameMode)))
    (Default|PressUILeft _asbp_game_mode_battle)))

(event Input|ActionEvents|InputActionUI_Cancel
  (params (Key :type Key%20Structure :default "None"))
  ;[1 1 1] UI
  (:Pressed
    (bind _asbp_game_mode_battle (Utilities|Casting|CastToBP_GameModeBattle (Game|GetGameMode)))
    (Default|PressUICancel _asbp_game_mode_battle)))

(event Input|ActionEvents|InputActionUI_OK
  (params (Key :type Key%20Structure :default "None"))
  ;[1 1 1] UI
  (:Pressed
    (Default|PressOK (Variables|Default|GetHero))))

(event Input|ActionEvents|InputActionAttack
  (params (Key :type Key%20Structure :default "None"))
  (:Pressed
    (if (Variables|/Game/Blueprints/BP_MyPlayerState.BP_MyPlayerState_C|GetBattleAble (Variables|Default|GetMyPlayerState))
      (Default|NormalAttack (Variables|Default|GetHero) 1))))

(event Input|ActionEvents|InputActionUI_SecondWeapon
  (params (Key :type Key%20Structure :default "None"))
  ;[1 1 1] UI
  (:Pressed
    (bind _asbp_game_mode_battle (Utilities|Casting|CastToBP_GameModeBattle (Game|GetGameMode)))
    (Default|UIPressSelectWeapon _asbp_game_mode_battle 2)))

(event Input|ActionEvents|InputActionShoot
  (params (Key :type Key%20Structure :default "None"))
  (:Pressed
    (if (Variables|/Game/Blueprints/BP_MyPlayerState.BP_MyPlayerState_C|GetBattleAble (Variables|Default|GetMyPlayerState))
      (if (Variables|ControlState|GetisAim)
        (Default|TryFireBall (Variables|Default|GetHero))))))

(event Input|ActionEvents|InputActionHeavyAttack
  (params (Key :type Key%20Structure :default "None"))
  (:Pressed
    (if (Variables|/Game/Blueprints/BP_MyPlayerState.BP_MyPlayerState_C|GetBattleAble (Variables|Default|GetMyPlayerState))
      (Default|NormalAttack (Variables|Default|GetHero) 2))))

(event Input|ActionEvents|InputActionWeaponSelect
  (params (Key :type Key%20Structure :default "None"))
  (:Pressed
    (Variables|ControlState|SetisWeaponSelectOpen true)
    (bind _asbp_game_mode_battle (Utilities|Casting|CastToBP_GameModeBattle (Game|GetGameMode)))
    (Default|OpenUIWeaponSelect _asbp_game_mode_battle)
    (Variables|/Game/Blueprints/BP_MyPlayerState.BP_MyPlayerState_C|SetBattleAble (Variables|Default|GetMyPlayerState) false))
  (:Released
    (Variables|ControlState|SetisWeaponSelectOpen false)
    (bind _asbp_game_mode_battle_2 (Utilities|Casting|CastToBP_GameModeBattle (Game|GetGameMode)))
    (Default|CloseUIWeaponSelect _asbp_game_mode_battle_2)
    (Variables|/Game/Blueprints/BP_MyPlayerState.BP_MyPlayerState_C|SetBattleAble (Variables|Default|GetMyPlayerState) true)))

(event Input|ActionEvents|InputActionUI_FirstWeapon
  (params (Key :type Key%20Structure :default "None"))
  ;[1 1 1] UI
  (:Pressed
    (bind _asbp_game_mode_battle (Utilities|Casting|CastToBP_GameModeBattle (Game|GetGameMode)))
    (Default|UIPressSelectWeapon _asbp_game_mode_battle 1)))

(event Input|ActionEvents|InputActionOpenMenu
  (params (Key :type Key%20Structure :default "None"))
  (:Pressed
    (Game|QuitGame 0 "Quit" false)))

(event Input|ActionEvents|InputActionUI_Map
  (params (Key :type Key%20Structure :default "None"))
  ;[1 1 1] UI
  (:Pressed
    (bind _asbp_game_mode_battle (Utilities|Casting|CastToBP_GameModeBattle (Game|GetGameMode)))
    (Default|OpenStageSelect _asbp_game_mode_battle)))

(event Input|ActionEvents|InputActionUI_UP
  (params (Key :type Key%20Structure :default "None"))
  ;[1 1 1] UI
  (:Pressed
    (bind _asbp_game_mode_battle (Utilities|Casting|CastToBP_GameModeBattle (Game|GetGameMode)))
    (Default|PressUIUp _asbp_game_mode_battle)))

(event Input|ActionEvents|InputActionUI_DOWN
  (params (Key :type Key%20Structure :default "None"))
  ;[1 1 1] UI
  (:Pressed
    (bind _asbp_game_mode_battle (Utilities|Casting|CastToBP_GameModeBattle (Game|GetGameMode)))
    (Default|PressUIDown _asbp_game_mode_battle)))

(event Input|ActionEvents|InputActionUI_Right
  (params (Key :type Key%20Structure :default "None"))
  ;[1 1 1] UI
  (:Pressed
    (bind _asbp_game_mode_battle (Utilities|Casting|CastToBP_GameModeBattle (Game|GetGameMode)))
    (Default|PressUIRight _asbp_game_mode_battle)))

(event Input|AxisEvents|InputAxisGoUp
  (params (AxisValue :type Float%20%28single-precision%29))
  (bind _returnvalue (Pawn|GetControlledPawn))
  (if (Variables|/Game/Blueprints/BP_MyPlayerState.BP_MyPlayerState_C|GetBattleAble (Variables|Default|GetMyPlayerState))
    (if (Variables|ControlState|GetisAim)
      (Pawn|Input|AddMovementInput _returnvalue "1.000000, 0, 0" (* AxisValue (Variables|Default|GetAimSpeed)) true)
      (else
        (Pawn|Input|AddMovementInput _returnvalue "1.000000, 0, 0" (* AxisValue (Variables|Default|GetSpeed)) true)))))

(event Input|AxisEvents|InputAxisGoRight
  (params (AxisValue :type Float%20%28single-precision%29))
  (bind _returnvalue (Pawn|GetControlledPawn))
  (if (Variables|/Game/Blueprints/BP_MyPlayerState.BP_MyPlayerState_C|GetBattleAble (Variables|Default|GetMyPlayerState))
    (if (Variables|ControlState|GetisAim)
      (Pawn|Input|AddMovementInput _returnvalue "0.000000,1.000000, 0" (* AxisValue (Variables|Default|GetAimSpeed)) true)
      (else
        (Pawn|Input|AddMovementInput _returnvalue "0.000000,1.000000, 0" (* AxisValue (Variables|Default|GetSpeed)) true)))))

(event Input|AxisEvents|InputAxisWeaponSelect_Right
  (params (AxisValue :type Float%20%28single-precision%29))
  ;[1 1 1] WeaponSelect
  (if (Variables|ControlState|GetisWeaponSelectOpen)
    (if (> (Math|Vector|VectorLength (Math|Vector|MakeVector AxisValue (stale Input|AxisEvents|InputAxisWeaponSelect_UP AxisValue) 0.0)) 0.15)
      (bind _asbp_game_mode_battle (Utilities|Casting|CastToBP_GameModeBattle (Game|GetGameMode)))
      (Default|UIWeaponAngle _asbp_game_mode_battle (+ (.yaw (Math|Conversions|RotationFromXVector (Math|Vector|MakeVector AxisValue (stale Input|AxisEvents|InputAxisWeaponSelect_UP AxisValue) 0.0))) 1.8e+02)))))

(event Input|AxisEvents|InputAxisWeaponSelect_UP
  (params (AxisValue :type Float%20%28single-precision%29))
  ;[1 1 1] WeaponSelect
  (if (Variables|ControlState|GetisWeaponSelectOpen)
    (if (> (Math|Vector|VectorLength (Math|Vector|MakeVector (stale Input|AxisEvents|InputAxisWeaponSelect_Right AxisValue) AxisValue 0.0)) 0.15)
      (bind _asbp_game_mode_battle (Utilities|Casting|CastToBP_GameModeBattle (Game|GetGameMode)))
      (Default|UIWeaponAngle _asbp_game_mode_battle (+ (.yaw (Math|Conversions|RotationFromXVector (Math|Vector|MakeVector (stale Input|AxisEvents|InputAxisWeaponSelect_Right AxisValue) AxisValue 0.0))) 1.8e+02)))))

(event Input|AxisEvents|InputAxisGoUp
  (params (AxisValue :type Float%20%28single-precision%29))
  (if (Variables|/Game/Blueprints/BP_MyPlayerState.BP_MyPlayerState_C|GetBattleAble (Variables|Default|GetMyPlayerState))
    (if (not (Variables|ControlState|GetisAim))
      (if (> (Math|Vector|VectorLength (Math|Vector|MakeVector AxisValue (stale Input|AxisEvents|InputAxisGoRight AxisValue) 0.0)) 0.15)
        (Pawn|SetControlRotation self (Math|Conversions|RotationFromXVector (Math|Vector|MakeVector AxisValue (stale Input|AxisEvents|InputAxisGoRight AxisValue) 0.0)))))))

(event Input|AxisEvents|InputAxisGoRight
  (params (AxisValue :type Float%20%28single-precision%29))
  (if (Variables|/Game/Blueprints/BP_MyPlayerState.BP_MyPlayerState_C|GetBattleAble (Variables|Default|GetMyPlayerState))
    (if (not (Variables|ControlState|GetisAim))
      (if (> (Math|Vector|VectorLength (Math|Vector|MakeVector (stale Input|AxisEvents|InputAxisGoUp AxisValue) AxisValue 0.0)) 0.15)
        (Pawn|SetControlRotation self (Math|Conversions|RotationFromXVector (Math|Vector|MakeVector (stale Input|AxisEvents|InputAxisGoUp AxisValue) AxisValue 0.0)))))))

(event Input|AxisEvents|InputAxisAimUp
  (params (AxisValue :type Float%20%28single-precision%29))
  (if (Variables|/Game/Blueprints/BP_MyPlayerState.BP_MyPlayerState_C|GetBattleAble (Variables|Default|GetMyPlayerState))
    (if (> (Math|Vector|VectorLength (Math|Vector|MakeVector AxisValue (stale Input|AxisEvents|InputAxisAimRight AxisValue) 0.0)) 0.1)
      (if (Variables|ControlState|GetisAim)
        _
        (else
          (Default|ShowAinHint (Variables|Default|GetHero))))
      (Variables|ControlState|SetisAim true)
      (Pawn|SetControlRotation self (Math|Conversions|RotationFromXVector (Math|Vector|MakeVector AxisValue (stale Input|AxisEvents|InputAxisAimRight AxisValue) 0.0)))
      (else
        (if (Variables|ControlState|GetisAim)
          (Default|HideAimHint (Variables|Default|GetHero)))
        (Variables|ControlState|SetisAim false)))))

(event Input|AxisEvents|InputAxisAimRight
  (params (AxisValue :type Float%20%28single-precision%29))
  (if (Variables|/Game/Blueprints/BP_MyPlayerState.BP_MyPlayerState_C|GetBattleAble (Variables|Default|GetMyPlayerState))
    (if (> (Math|Vector|VectorLength (Math|Vector|MakeVector (stale Input|AxisEvents|InputAxisAimUp AxisValue) AxisValue 0.0)) 0.1)
      (if (Variables|ControlState|GetisAim)
        _
        (else
          (Default|ShowAinHint (Variables|Default|GetHero))))
      (Variables|ControlState|SetisAim true)
      (Pawn|SetControlRotation self (Math|Conversions|RotationFromXVector (Math|Vector|MakeVector (stale Input|AxisEvents|InputAxisAimUp AxisValue) AxisValue 0.0)))
      (else
        (if (Variables|ControlState|GetisAim)
          (Default|HideAimHint (Variables|Default|GetHero)))
        (Variables|ControlState|SetisAim false)))))

(fn ConstructionScript)