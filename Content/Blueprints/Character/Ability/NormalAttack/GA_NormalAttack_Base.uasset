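; Base Gameplay Ability for a hero's normal attack, which updates the hero's combo and plays the attack montage.
; On each deal-damage gameplay event, it applies a damage effect to the event target, scaled by the hero's combo damage level.
; Each hit also plays a sound and pushes the target away from the attacker with a brief stun.
; The ability ends when the montage completes, blends out, or is interrupted or cancelled.
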(event Ability|EventActivateAbility
  (Ability|CommitAbility)
  (bind _asbp_hero_unit (Utilities|Casting|CastToBP_HeroUnit (Ability|GetOwningActorfromActorInfo)))
  (Default|DeterminCombo _asbp_hero_unit)
  (|PlayMontageandWaitProxy "None" (Variables|AbilityData|GetSkillMontage) 1.0 "None" true 1.0
    (:then
      (bind _payload (Ability|Tasks|WaitGameplayEvent "(TagName=\"skill.NormalAttack.dealDamage\")" 0)
        (:EventReceived
          (GameplayEffects|ApplyGameplayEffectToTarget (Ability|TargetData|AbilityTargetDatafromActor (.Target (Utilities|Struct|BreakGameplayEventData _payload))) (Variables|AbilityData|GetGE_Class) (Variables|/Game/Blueprints/Character/BP_CharacterBase.BP_CharacterBase_C|GetComboDamageLevel _asbp_hero_unit) 1)
          (Audio|PlaySound2D "/Game/Audio/Sound/SND_BTL_HIT_01.SND_BTL_HIT_01" 0.5 1.0 0.0 0 0)
          (bind _asbp_character_base (Utilities|Casting|CastToBP_CharacterBase (.Target (Utilities|Struct|BreakGameplayEventData _payload))))
          (Default|PushCharacter _asbp_character_base (Math|Vector|Normalize (- (Transformation|GetActorLocation _asbp_character_base) (Transformation|GetActorLocation (Ability|GetOwningActorfromActorInfo)))) 3e+02 1.0))))
    (:OnCompleted
      (Ability|EndAbility :!label _label))
    (:OnBlendOut
      (goto _label))
    (:OnInterrupted
      (goto _label))
    (:OnCancelled
      (goto _label))))

(event Ability|EventOnEndAbility
  (params (bWasCancelled :type Boolean)))