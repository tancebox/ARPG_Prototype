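; Gameplay ability for the EM normal attack, a combo attack that damages and pushes the characters it hits.
; On activation it commits, has the owning BP_CharacterBase determine the combo and plays that character's attack montage.
; Each dealDamage gameplay event applies the damage effect at the combo damage level, then pushes the target away from the attacker without stun.
; The ability ends when the montage completes, blends out or is interrupted or cancelled.
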(event Ability|EventActivateAbility
  (Ability|CommitAbility)
  (bind _asbp_character_base (Utilities|Casting|CastToBP_CharacterBase (Ability|GetOwningActorfromActorInfo)))
  (Default|DeterminCombo _asbp_character_base)
  (|PlayMontageandWaitProxy "None" (Variables|/Game/Blueprints/Character/BP_CharacterBase.BP_CharacterBase_C|GetAttackMontage _asbp_character_base) 1.0 "None" true 1.0
    (:then
      (bind _payload (Ability|Tasks|WaitGameplayEvent "(TagName=\"skill.NormalAttack.dealDamage\")" 0)
        (:EventReceived
          (GameplayEffects|ApplyGameplayEffectToTarget (Ability|TargetData|AbilityTargetDatafromActor (.Target (Utilities|Struct|BreakGameplayEventData _payload))) "/Game/Blueprints/Character/Ability/NormalAttack/GE_EMNormalAttack_Damage.GE_EMNormalAttack_Damage_C" (Variables|/Game/Blueprints/Character/BP_CharacterBase.BP_CharacterBase_C|GetComboDamageLevel _asbp_character_base) 1)
          (bind _asbp_character_base_2 (Utilities|Casting|CastToBP_CharacterBase (.Target (Utilities|Struct|BreakGameplayEventData _payload))))
          (Default|PushCharacter _asbp_character_base_2 (Math|Vector|Normalize (- (Transformation|GetActorLocation _asbp_character_base_2) (Transformation|GetActorLocation (Ability|GetOwningActorfromActorInfo)))) 1e+02 0.0))))
    (:OnCompleted
      (Ability|EndAbility :!label _label))
    (:OnBlendOut
      (goto _label))
    (:OnInterrupted
      (goto _label))
    (:OnCancelled
      (goto _label))))

(event Ability|EventOnEndAbility
  (params (bWasCancelled :type Boolean)))