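; Gameplay ability for a dash that launches the character forward, damaging, pushing and stunning targets it hits.
; On activation it commits, starts the UI cooldown, zeroes ground friction, applies a velocity-change impulse and sets pawn collision to overlap during the dash montage.
; A gameplay event supplies each target for the damage effect and knockback away from the owner.
; Montage exits restore friction and collision, with friction also restored on ability end.
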(event Ability|EventActivateAbility
  (Ability|CommitAbility)
  (CallFunction|DoUICooldown)
  (bind _ascharacter (Utilities|Casting|CastToCharacter (Ability|GetOwningActorfromActorInfo))
    (:then
      (Variables|Default|SetOriginalGroundFiction (Variables|/Script/Engine.CharacterMovementComponent|GetGroundFriction (Variables|/Script/Engine.Character|GetCharacterMovement _ascharacter)))
      (Variables|/Script/Engine.CharacterMovementComponent|SetGroundFriction (Variables|/Script/Engine.Character|GetCharacterMovement _ascharacter) 0.0)
      (Physics|AddImpulse (Variables|/Script/Engine.Character|GetCharacterMovement _ascharacter) (* (Transformation|GetActorForwardVector _ascharacter) 1e+03) true)
      (bind _characterbase (CallFunction|GetCharacterandController))
      (Default|SetCollisiontoPawn _characterbase "ECR_Overlap")
      (|PlayMontageandWaitProxy "None" "/Game/Blueprints/Character/Animation/AM_Dash.AM_Dash" 1.0 "None" true 1.0
        (:then
          (bind _payload (Ability|Tasks|WaitGameplayEvent "(TagName=\"skill.dash.dealDamage\")" 0)
            (:EventReceived
              (GameplayEffects|ApplyGameplayEffectToTarget (Ability|TargetData|AbilityTargetDatafromActor (.Target (Utilities|Struct|BreakGameplayEventData _payload))) "/Game/Blueprints/Character/Ability/Dash/GE_Dash_Damage.GE_Dash_Damage_C" 1 1)
              (bind _asbp_character_base (Utilities|Casting|CastToBP_CharacterBase (.Target (Utilities|Struct|BreakGameplayEventData _payload))))
              (Default|PushCharacter _asbp_character_base (Math|Vector|Normalize (- (Transformation|GetActorLocation _asbp_character_base) (Transformation|GetActorLocation (Ability|GetOwningActorfromActorInfo)))) 2e+03 5.0))))
        (:OnCompleted
          (Variables|/Script/Engine.CharacterMovementComponent|SetGroundFriction (Variables|/Script/Engine.Character|GetCharacterMovement _ascharacter) (Variables|Default|GetOriginalGroundFiction) :!label _label)
          (bind _characterbase_2 (CallFunction|GetCharacterandController))
          (Default|SetCollisiontoPawn _characterbase_2 "ECR_Block")
          (Ability|EndAbility))
        (:OnBlendOut
          (goto _label))
        (:OnInterrupted
          (goto _label))
        (:OnCancelled
          (goto _label))))
    (:CastFailed
      (Ability|EndAbility))))

(event Ability|EventOnEndAbility
  (params (bWasCancelled :type Boolean))
  (bind _ascharacter (Utilities|Casting|CastToCharacter (Ability|GetOwningActorfromActorInfo)))
  (Variables|/Script/Engine.CharacterMovementComponent|SetGroundFriction (Variables|/Script/Engine.Character|GetCharacterMovement _ascharacter) (Variables|Default|GetOriginalGroundFiction)))