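; Gameplay ability that dashes the owning Character forward.
; On activation it commits, zeroes the movement component's ground friction and applies a velocity-change impulse along the actor's forward vector.
; It plays the dash montage, then restores the saved friction and ends when the montage completes, blends out, is interrupted or is cancelled.
; The commit result is unchecked, and friction is restored only through those montage callbacks.
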(event Ability|EventActivateAbility
  (Ability|CommitAbility)
  (bind _ascharacter (Utilities|Casting|CastToCharacter (Ability|GetOwningActorfromActorInfo))
    (:then
      (Variables|Default|SetOriginalGroundFiction (Variables|/Script/Engine.CharacterMovementComponent|GetGroundFriction (Variables|/Script/Engine.Character|GetCharacterMovement _ascharacter)))
      (Variables|/Script/Engine.CharacterMovementComponent|SetGroundFriction (Variables|/Script/Engine.Character|GetCharacterMovement _ascharacter) 0.0)
      (Physics|AddImpulse (Variables|/Script/Engine.Character|GetCharacterMovement _ascharacter) (* (Transformation|GetActorForwardVector _ascharacter) 1e+03) true)
      (|PlayMontageandWaitProxy "None" "/Game/Blueprints/Character/Animation/AM_Dash.AM_Dash" 1.0 "None" true 1.0
        (:OnCompleted
          _)
        (:OnBlendOut
          _)
        (:OnInterrupted
          _)
        (:OnCancelled
          _))
      (Variables|/Script/Engine.CharacterMovementComponent|SetGroundFriction (Variables|/Script/Engine.Character|GetCharacterMovement _ascharacter) (Variables|Default|GetOriginalGroundFiction))
      (Ability|EndAbility))
    (:CastFailed
      (Ability|EndAbility))))

(event Ability|EventOnEndAbility
  (params (bWasCancelled :type Boolean)))