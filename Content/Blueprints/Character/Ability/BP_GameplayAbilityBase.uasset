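; Base Gameplay Ability Blueprint that provides shared helpers for character abilities, with no activation logic of its own.
; It resolves the owning character and player controller, and starts the cooldown on primary UI slots matching its ability class.
; A cost check compares the negated AbilityInfo cost against player zero's attribute for the cost type, printing debug strings.
; The Health case reads Mana instead of health.
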(event Ability|EventActivateAbility)

(event Ability|EventOnEndAbility
  (params (bWasCancelled :type Boolean)))

(fn GetCharacterandController
  (bind _asbp_character_base (Utilities|Casting|CastToBP_CharacterBase (Ability|GetOwningActorfromActorInfo)))
  (bind _asbp_player_controller (Utilities|Casting|CastToBP_PlayerController (Pawn|GetController _asbp_character_base))
    (:then
      _)
    (:CastFailed
      _))
  (return _asbp_character_base _asbp_player_controller))

(fn DoUICooldown
  (bind _asbp_player_controller (Utilities|Casting|CastToBP_PlayerController (Game|GetPlayerController 0)))
  (Utilities|IsValid _asbp_player_controller
    (:Is%20Valid
      (for _array_element (Variables|/Game/UI/WBP_PrimaryUI.WBP_PrimaryUI_C|GetSlots (Variables|/Game/Blueprints/Character/BP_PlayerController.BP_PlayerController_C|GetPrimaryUI _asbp_player_controller))
        (bind _returnvalue (Class|GameplayAbilityBase|GetAbilityInfo))
        (if (== (.abilityclass (Variables|/Game/UI/WBP_Ability_Slot.WBP_Ability_Slot_C|GetAbilityInfo _array_element)) (.abilityclass _returnvalue))
          (Default|StartCooldown _array_element))))))

(fn IsCostStillAvailable
  (bind _returnvalue (Class|GameplayAbilityBase|GetAbilityInfo))
  (LocalVariables|Setcost (* (.cost _returnvalue) -1.0))
  (switch Utilities|FlowControl|Switch|SwitchonEAbilityCostType (.costtype _returnvalue)
    (:Health
      (Development|PrintString "H")
      (bind _ascharacter_base (Utilities|Casting|CastToCharacterBase (Game|GetPlayerCharacter 0)))
      (return (> (.currentvalue (Variables|/Script/ProjectARPG.AttributeSetBase|GetMana (Variables|/Script/ProjectARPG.CharacterBase|GetAttributeSetBaseComp _ascharacter_base))) (LocalVariables|Getcost))))
    (:Mana
      (Development|PrintString "M")
      (bind _asbp_character_base (Utilities|Casting|CastToBP_CharacterBase (Game|GetPlayerCharacter 0)))
      (Development|PrintString (Utilities|String|ToString(Boolean) (> (.currentvalue (Variables|/Script/ProjectARPG.AttributeSetBase|GetMana (Variables|/Script/ProjectARPG.CharacterBase|GetAttributeSetBaseComp _asbp_character_base))) (LocalVariables|Getcost))))
      (return (> (.currentvalue (Variables|/Script/ProjectARPG.AttributeSetBase|GetMana (Variables|/Script/ProjectARPG.CharacterBase|GetAttributeSetBaseComp _asbp_character_base))) (LocalVariables|Getcost))))
    (:Strength
      (Development|PrintString "S")
      (bind _ascharacter_base_2 (Utilities|Casting|CastToCharacterBase (Game|GetPlayerCharacter 0)))
      (return (> (.currentvalue (Variables|/Script/ProjectARPG.AttributeSetBase|GetStrength (Variables|/Script/ProjectARPG.CharacterBase|GetAttributeSetBaseComp _ascharacter_base_2))) (LocalVariables|Getcost))))))