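; BP_FireBall is a fireball ability actor that applies a gameplay effect to hostile characters it touches.
; On sphere overlap, it casts the other actor and its instigator to BP_CharacterBase and checks hostility.
; For a hostile target, the instigator applies the stored ability effect spec through target data, then the fireball plays a sound and destroys itself.
; A timer started at BeginPlay also destroys it after a fixed lifetime.
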(event OnComponentBeginOverlap(Sphere)
  (params (OverlappedComponent :type Primitive%20Component%20Object%20Reference) (OtherActor :type Actor%20Object%20Reference) (OtherComp :type Primitive%20Component%20Object%20Reference) (OtherBodyIndex :type Integer) (bFromSweep :type Boolean) (SweepResult :type Hit%20Result%20Structure%20%28by%20ref%29))
  (bind _asbp_character_base (Utilities|Casting|CastToBP_CharacterBase OtherActor))
  (bind _asbp_character_base_2 (Utilities|Casting|CastToBP_CharacterBase (Game|GetInstigator)))
  (bind _returnvalue (Class|CharacterBase|IsOtherHostile _asbp_character_base _asbp_character_base_2))
  (if _returnvalue
    (Class|CharacterBase|ApplyGESpecHandletoTargetDataSpecHandle _asbp_character_base_2 (Variables|Default|GetEffectSpecHandleFromAbility) (Ability|TargetData|AbilityTargetDatafromActor _asbp_character_base))
    (Audio|PlaySound2D "/Game/Audio/Sound/SND_BTL_FIRE_BOLT_02.SND_BTL_FIRE_BOLT_02" 1.0 1.0 0.0 0 0)
    (Actor|DestroyActor)))

(event Custom|TimeToDIE
  (Actor|DestroyActor))

(event EventBeginPlay
  (Utilities|Time|SetTimerbyEvent (delegate Custom|TimeToDIE) 6.0))

(event Collision|EventActorBeginOverlap
  (params (OtherActor :type Actor%20Object%20Reference)))

(event EventTick
  (params (DeltaSeconds :type Float%20%28single-precision%29)))

(fn ConstructionScript)