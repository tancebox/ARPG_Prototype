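; Gameplay ability that fires a fireball from the owning CharacterBase.
; It commits, plays a ranger attack montage and, on a montage notify, spawns BP_EM_FireBall at the character's transform, then ends.
; The projectile receives an outgoing GE_Dash_Damage spec and the character as instigator.
; Completion, blend-out or interruption just ends the ability; an unconnected PlayMontageAndWait variant that spawns on completion never runs.
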(event Ability|EventActivateAbility
  (Ability|CommitAbility)
  (Animation|Montage|PlayMontage (Variables|/Script/Engine.Character|GetMesh (.AsCharacter%20Base (Utilities|Casting|CastToCharacterBase (Ability|GetOwningActorfromActorInfo)))) "/Game/Blueprints/Character/Animation/AM_EM_RangerAttack_01.AM_EM_RangerAttack_01"
    (:OnCompleted
      (Ability|EndAbility :!label _label))
    (:OnBlendOut
      (goto _label))
    (:OnInterrupted
      (goto _label))
    (:OnNotifyBegin
      (bind _ascharacter_base (Utilities|Casting|CastToCharacterBase (Ability|GetOwningActorfromActorInfo)))
      (Game|SpawnActorfromClass "/Game/Blueprints/Character/Ability/FireBall/BP_EM_FireBall.BP_EM_FireBall_C" (Transformation|GetActorTransform _ascharacter_base) "AlwaysSpawn" 0 (Ability|MakeOutgoingGameplayEffectSpec "/Game/Blueprints/Character/Ability/Dash/GE_Dash_Damage.GE_Dash_Damage_C") _ascharacter_base)
      (Ability|EndAbility))))

(event Ability|EventOnEndAbility
  (params (bWasCancelled :type Boolean)))