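; BP_NPC is a talkable NPC that shows a talk hint while an overlap is active on its sphere.
; Overlap begin registers it as the focus NPC on BP_GameModeBattle, and overlap end clears that focus, with no check on the overlapping actor.
; StartTalk copies the NPC's name and dialogue text into the game mode's shared UIFullTalk widget and shows it.
; EndTalk hides that widget.
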(event OnComponentBeginOverlap(Sphere)
  (params (OverlappedComponent :type Primitive%20Component%20Object%20Reference) (OtherActor :type Actor%20Object%20Reference) (OtherComp :type Primitive%20Component%20Object%20Reference) (OtherBodyIndex :type Integer) (bFromSweep :type Boolean) (SweepResult :type Hit%20Result%20Structure%20%28by%20ref%29))
  (Default|SetFocusNPC (.AsBP%20Game%20Mode%20Battle (Utilities|Casting|CastToBP_GameModeBattle (Game|GetGameMode))) self)
  (Rendering|SetVisibility (Variables|Default|GetTalkHint) true false))

(event OnComponentEndOverlap(Sphere)
  (params (OverlappedComponent :type Primitive%20Component%20Object%20Reference) (OtherActor :type Actor%20Object%20Reference) (OtherComp :type Primitive%20Component%20Object%20Reference) (OtherBodyIndex :type Integer))
  (Default|ClearFocusNPC (.AsBP%20Game%20Mode%20Battle (Utilities|Casting|CastToBP_GameModeBattle (Game|GetGameMode))))
  (Rendering|SetVisibility (Variables|Default|GetTalkHint) false false))

(event Custom|StartTalk
  (bind _returnvalue (Game|GetGameMode))
  (bind _asbp_game_mode_battle (Utilities|Casting|CastToBP_GameModeBattle _returnvalue))
  (bind _ui_fulltalk (Variables|/Game/Blueprints/BP_GameModeBattle.BP_GameModeBattle_C|GetUI_FullTalk _asbp_game_mode_battle))
  (Rendering|Components|TextRender|SetText (Variables|/Game/UI/NPC/WBP_FullTalk.WBP_FullTalk_C|GetTalkContent _ui_fulltalk) (Variables|Default|GetTalkContent))
  (Rendering|Components|TextRender|SetText (Variables|/Game/UI/NPC/WBP_FullTalk.WBP_FullTalk_C|GetTextBlock_Name _ui_fulltalk) (Variables|Default|GetTalkName))
  (Widget|SetVisibility _ui_fulltalk "Visible"))

(event Custom|EndTalk
  (Widget|SetVisibility (Variables|/Game/Blueprints/BP_GameModeBattle.BP_GameModeBattle_C|GetUI_FullTalk (.AsBP%20Game%20Mode%20Battle (Utilities|Casting|CastToBP_GameModeBattle (Game|GetGameMode)))) "Hidden"))

(event EventBeginPlay
  (|CallParentFunction)
  (Rendering|SetVisibility (Variables|Default|GetTalkHint) false false))

(event Collision|EventActorBeginOverlap
  (params (OtherActor :type Actor%20Object%20Reference))
  (|CallParentFunction OtherActor) ; This node is disabled and will not be called.\nDrag off pins to build functionality.
)

(event EventTick
  (params (DeltaSeconds :type Float%20%28single-precision%29))
  (|CallParentFunction DeltaSeconds) ; This node is disabled and will not be called.\nDrag off pins to build functionality.
)

(fn ConstructionScript
  (|CallParentFunction))