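; Base character Blueprint for GAS-driven combat, providing melee and dash hit detection, knockback and combo state.
; Weapon and capsule overlaps check hostility, then send damage gameplay events to itself with the target as payload; dash hits use an exclusion list to avoid repeats.
; PushCharacter briefly zeroes ground friction around an impulse, with optional stun.
; Helpers toggle Pawn collision and rotation mode, cycle a three-step montage combo, and load saved HP.
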(event OnComponentBeginOverlap(WeaponCollider)
  (params (OverlappedComponent :type Primitive%20Component%20Object%20Reference) (OtherActor :type Actor%20Object%20Reference) (OtherComp :type Primitive%20Component%20Object%20Reference) (OtherBodyIndex :type Integer) (bFromSweep :type Boolean) (SweepResult :type Hit%20Result%20Structure%20%28by%20ref%29))
  (if (!= self OtherActor)
    (bind _ascharacter_base (Utilities|Casting|CastToCharacterBase OtherActor))
    (bind _returnvalue (Class|CharacterBase|IsOtherHostile _ascharacter_base self))
    (if _returnvalue
      (Ability|SendGameplayEventtoActor self "(TagName=\"skill.NormalAttack.dealDamage\")" (Utilities|Struct|MakeGameplayEventData "" 0 OtherActor)))))

(event OnComponentBeginOverlap(CapsuleComponent)
  (params (OverlappedComponent :type Primitive%20Component%20Object%20Reference) (OtherActor :type Actor%20Object%20Reference) (OtherComp :type Primitive%20Component%20Object%20Reference) (OtherBodyIndex :type Integer) (bFromSweep :type Boolean) (SweepResult :type Hit%20Result%20Structure%20%28by%20ref%29))
  (bind _self self)
  ;[1 1 1] Dash Overlap
  (bind _asbp_character_base (Utilities|Casting|CastToBP_CharacterBase OtherActor))
  (bind _returnvalue (Class|CharacterBase|IsOtherHostile _asbp_character_base _self))
  (if _returnvalue
    (if (not (Utilities|Array|ContainsItem (Variables|Default|GetOverlapExeclide) _asbp_character_base))
      (Utilities|Array|AddUnique (Variables|Default|GetOverlapExeclide) _asbp_character_base)
      (Ability|SendGameplayEventtoActor self "(TagName=\"skill.dash.dealDamage\")" (Utilities|Struct|MakeGameplayEventData "" _self OtherActor)))))

(event Custom|PushCharacter
  (params (ImpulseDirection :type Vector) (PushStrength :type Float%20%28single-precision%29) (StunDuration :type Float%20%28single-precision%29))
  (bind _charactermovement (Variables|Character|GetCharacterMovement))
  (Variables|Default|SetDefaultGroundFriction (Variables|/Script/Engine.CharacterMovementComponent|GetGroundFriction _charactermovement))
  (Variables|/Script/Engine.CharacterMovementComponent|SetGroundFriction _charactermovement 0.0)
  (Physics|AddImpulse (Variables|Character|GetCharacterMovement) (* ImpulseDirection PushStrength) true)
  (if (> StunDuration 0.0)
    (Class|CharacterBase|HitStun StunDuration))
  (Utilities|FlowControl|Delay 0.3)
  (Variables|/Script/Engine.CharacterMovementComponent|SetGroundFriction (Variables|Character|GetCharacterMovement) (Variables|Default|GetDefaultGroundFriction)))

(event Custom|MakeCameraControlRotation
  (params (ShouldControlRotation :type Boolean))
  ;[1 1 1] 這個應該用不到
  (if ShouldControlRotation
    (Variables|Default|SetbUseControllerRotationYaw true)
    (Variables|/Script/Engine.CharacterMovementComponent|SetbOrientRotationToMovement (Variables|Character|GetCharacterMovement) false)
    (else
      (Variables|Default|SetbUseControllerRotationYaw false)
      (Variables|/Script/Engine.CharacterMovementComponent|SetbOrientRotationToMovement (Variables|Character|GetCharacterMovement) true))))

(event Custom|ResetComboCount
  (Variables|Default|SetComboCount 1))

(event Custom|SetUnitAttrFromSave
  (bind _returnvalue (SaveGame|LoadGamefromSlot (Variables|/Game/Blueprints/BP_MyGameInstance.BP_MyGameInstance_C|GetCurrentSaveSlotName (.AsBP%20My%20Game%20Instance (Utilities|Casting|CastToBP_MyGameInstance (Game|GetGameInstance))))))
  (bind _asbp_save_game (Utilities|Casting|CastToBP_SaveGame _returnvalue))
  (Class|AttributeSetBase|SetActorHealth (Variables|Default|GetAttributeSetBaseComp) (.hp (Variables|/Game/Blueprints/System/BP_SaveGame.BP_SaveGame_C|GetUnitAttribute _asbp_save_game)))
  (CallFunction|TempPrintHP))

(event Custom|tempPrintHP
  (Development|PrintString (Utilities|String|ToString(Float) (.basevalue (Variables|/Script/ProjectARPG.AttributeSetBase|GetMaxHealth (Variables|Default|GetAttributeSetBaseComp))))))

(event EventBeginPlay)

(event Collision|EventActorBeginOverlap
  (params (OtherActor :type Actor%20Object%20Reference)))

(event EventTick
  (params (DeltaSeconds :type Float%20%28single-precision%29)))

(event EventDie)

(fn ConstructionScript)

(fn SetCollisiontoPawn
  (params (NewResponse :type ECollisionResponse%20Enum :default "ECR_Ignore"))
  (Collision|SetCollisionResponsetoChannel (Variables|Default|GetCapsuleComponent) "ECC_Pawn" NewResponse))

(fn DeterminComboOld
  (switch int (Variables|Default|GetComboCount)
    (:1
      (Variables|Default|SetComboCount 2)
      (bind _output_get (Variables|Default|SetComboDamageLevel 1))
      (Variables|Default|SetAttackMontage "/Game/Blueprints/Character/Animation/AM_NormalAttack_01.AM_NormalAttack_01")
      (return _output_get))
    (:2
      (Variables|Default|SetComboCount 3)
      (bind _output_get_2 (Variables|Default|SetComboDamageLevel 2))
      (Variables|Default|SetAttackMontage "/Game/Blueprints/Character/Animation/AM_NormalAttack_02.AM_NormalAttack_02")
      (return _output_get_2))
    (:3
      (Variables|Default|SetComboCount 1)
      (bind _output_get_3 (Variables|Default|SetComboDamageLevel 3))
      (Variables|Default|SetAttackMontage "/Game/Blueprints/Character/Animation/AM_NormalAttack_03.AM_NormalAttack_03")
      (return _output_get_3))))