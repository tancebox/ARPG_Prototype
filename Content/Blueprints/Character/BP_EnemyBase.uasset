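; BP_EnemyBase is an enemy character Blueprint that handles its attack, health display and death.
; NormalAttack activates the GA_EM_NormalAttack gameplay ability through its Ability System Component.
; Health changes update a HealthBar widget component with the current health ratio.
; Die plays a death sound and montage, then destroys the actor after a one-second delay.
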(event Custom|NormalAttack
  (Abilities|TryActivateAbilitybyClass (Variables|Default|GetAbilitySystemComp) "/Game/Blueprints/Character/Ability/NormalAttack/GA_EM_NormalAttack.GA_EM_NormalAttack_C" true))

(event EventBeginPlay
  (|CallParentFunction))

(event Collision|EventActorBeginOverlap
  (params (OtherActor :type Actor%20Object%20Reference))
  (|CallParentFunction OtherActor) ; This node is disabled and will not be called.\nDrag off pins to build functionality.
)

(event EventTick
  (params (DeltaSeconds :type Float%20%28single-precision%29))
  (|CallParentFunction DeltaSeconds) ; This node is disabled and will not be called.\nDrag off pins to build functionality.
)

(event EventDie
  (Audio|PlaySound2D "/Game/Audio/Sound/SND_BTL_DEAD_01.SND_BTL_DEAD_01" 1.0 1.0 0.0 0 0)
  (Animation|PlayAnimMontage "/Game/Blueprints/Character/AM_Die.AM_Die" 1.0 "None")
  (Utilities|FlowControl|Delay 1.0)
  (Actor|DestroyActor))

(event EventOnHealthChanged
  (params (Health :type Float%20%28single-precision%29) (MaxHealth :type Float%20%28single-precision%29))
  (bind _ashealth_bar (Utilities|Casting|CastToHealthBar (UserInterface|GetUserWidgetObject (Variables|Default|GetHealthBar))))
  (Default|SetPercentage _ashealth_bar (/ Health MaxHealth)))

(fn ConstructionScript
  (|CallParentFunction))