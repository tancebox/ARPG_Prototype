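; Ranger enemy character Blueprint that uses the Gameplay Ability System for its ranged fireball skill.
; On BeginPlay it runs the parent logic, then acquires the abilities listed in InitialAbilities.
; The NormalSkill event activates GA_EM_FireBall by class through the ability system component, with remote activation allowed.
; Overlap, tick and construction add no logic of their own.
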(event Custom|NormalSkill
  (Abilities|TryActivateAbilitybyClass (Variables|Default|GetAbilitySystemComp) "/Game/Blueprints/Character/Ability/FireBall/GA_EM_FireBall.GA_EM_FireBall_C" true))

(event EventBeginPlay
  (|CallParentFunction)
  (Class|CharacterBase|AquireAbilities (Variables|Default|GetInitialAbilities)))

(event Collision|EventActorBeginOverlap
  (params (OtherActor :type Actor%20Object%20Reference))
  (|CallParentFunction OtherActor) ; This node is disabled and will not be called.\nDrag off pins to build functionality.
)

(event EventTick
  (params (DeltaSeconds :type Float%20%28single-precision%29))
  (|CallParentFunction DeltaSeconds) ; This node is disabled and will not be called.\nDrag off pins to build functionality.
)

(fn ConstructionScript
  (|CallParentFunction))