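; Save point actor that shows a save hint near the hero and writes game progress.
; Sphere overlaps, meant for BP_HeroUnit, toggle the hint through BP_GameModeBattle, which also receives this point as its focused save point.
; SaveGame overwrites only an existing current slot with a fresh BP_SaveGame holding player max health and the target level and position, then calls the game instance's SaveGame.
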(event OnComponentBeginOverlap(Sphere)
  (params (OverlappedComponent :type Primitive%20Component%20Object%20Reference) (OtherActor :type Actor%20Object%20Reference) (OtherComp :type Primitive%20Component%20Object%20Reference) (OtherBodyIndex :type Integer) (bFromSweep :type Boolean) (SweepResult :type Hit%20Result%20Structure%20%28by%20ref%29))
  (bind _returnvalue (Game|GetGameMode))
  (bind _asbp_game_mode_battle (Utilities|Casting|CastToBP_GameModeBattle _returnvalue))
  (if (== (Utilities|GetClass 0) "/Game/Blueprints/Character/BP_HeroUnit.BP_HeroUnit_C")
    (Default|OpenUISaveHint _asbp_game_mode_battle)
    (Default|SetFocusSavePoint _asbp_game_mode_battle self)))

(event OnComponentEndOverlap(Sphere)
  (params (OverlappedComponent :type Primitive%20Component%20Object%20Reference) (OtherActor :type Actor%20Object%20Reference) (OtherComp :type Primitive%20Component%20Object%20Reference) (OtherBodyIndex :type Integer))
  (if (== (Utilities|GetClass 0) "/Game/Blueprints/Character/BP_HeroUnit.BP_HeroUnit_C")
    (Default|CloseUISaveHint (.AsBP%20Game%20Mode%20Battle (Utilities|Casting|CastToBP_GameModeBattle (Game|GetGameMode))))))

(event Custom|SaveGame
  (bind _asbp_my_game_instance (Utilities|Casting|CastToBP_MyGameInstance (Game|GetGameInstance)))
  (bind _returnvalue (SaveGame|DoesSaveGameExist (Variables|/Game/Blueprints/BP_MyGameInstance.BP_MyGameInstance_C|GetCurrentSaveSlotName _asbp_my_game_instance)))
  (if _returnvalue
    (Development|PrintString "YES")
    (bind _returnvalue_2 (SaveGame|CreateSaveGameObject "/Game/Blueprints/System/BP_SaveGame.BP_SaveGame_C"))
    (Variables|/Game/Blueprints/System/BP_SaveGame.BP_SaveGame_C|SetUnitAttribute _returnvalue_2 (Utilities|Struct|MakeST_UnitAttr (.basevalue (Variables|/Script/ProjectARPG.AttributeSetBase|GetMaxHealth (Variables|/Script/ProjectARPG.CharacterBase|GetAttributeSetBaseComp (.AsBP%20Character%20Base (Utilities|Casting|CastToBP_CharacterBase (Game|GetPlayerCharacter 0)))))) 0.0))
    (Variables|/Game/Blueprints/System/BP_SaveGame.BP_SaveGame_C|SetLevelName _returnvalue_2 (Variables|Default|GetTargetLevelName))
    (Variables|/Game/Blueprints/System/BP_SaveGame.BP_SaveGame_C|SetPosition _returnvalue_2 (Variables|Default|GetTargetPosition))
    (bind _asbp_my_game_instance_2 (Utilities|Casting|CastToBP_MyGameInstance (Game|GetGameInstance)))
    (SaveGame|SaveGametoSlot _returnvalue_2 (Variables|/Game/Blueprints/BP_MyGameInstance.BP_MyGameInstance_C|GetCurrentSaveSlotName _asbp_my_game_instance_2))
    (Default|SaveGame (.AsBP%20My%20Game%20Instance (Utilities|Casting|CastToBP_MyGameInstance (Game|GetGameInstance))))
    (else
      (Development|PrintString "NO"))))

(event EventBeginPlay)

(event Collision|EventActorBeginOverlap
  (params (OtherActor :type Actor%20Object%20Reference)))

(event EventTick
  (params (DeltaSeconds :type Float%20%28single-precision%29)))

(fn ConstructionScript)