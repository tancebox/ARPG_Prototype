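; Game instance Blueprint that serves as the entry point for saving and loading the game through a BP_SaveSystem actor.
; SetUpSaveSystem spawns that actor at the origin and stores it if no valid reference exists.
; SaveGame uses the stored actor or spawns an unstored temporary reference when it is invalid.
; LoadGame forwards the slot name to the stored actor without a validity check.
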(event Custom|SaveGame
  (bind _savesystem (Variables|Default|GetSaveSystem))
  (Utilities|IsValid _savesystem
    (:Is%20Valid
      (Default|SaveGame _savesystem))
    (:Is%20Not%20Valid
      (bind _returnvalue (Game|SpawnActorfromClass "/Game/Blueprints/System/BP_SaveSystem.BP_SaveSystem_C" (Math|Transform|MakeTransform "0, 0, 0") "Undefined" 0 0))
      (Default|SaveGame _returnvalue))))

(event Custom|LoadGame
  (params (SaveSlotName :type String))
  (Default|LoadGame (Variables|Default|GetSaveSystem) SaveSlotName))

(event Custom|SetUpSaveSystem
  (Utilities|IsValid (Variables|Default|GetSaveSystem)
    (:Is%20Not%20Valid
      (bind _returnvalue (Game|SpawnActorfromClass "/Game/Blueprints/System/BP_SaveSystem.BP_SaveSystem_C" (Math|Transform|MakeTransform "0, 0, 0") "Undefined" 0 0))
      (Variables|Default|SetSaveSystem _returnvalue))))