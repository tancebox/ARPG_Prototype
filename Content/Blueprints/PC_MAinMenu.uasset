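; Player controller for the main menu that routes menu input to the game mode.
; On each OK, Up, Down and Cancel UI action press, it casts the current game mode to GM_MainMenu and calls the matching Press function.
; It holds no menu logic itself, and BeginPlay, Tick and the construction script are empty.
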(event EventBeginPlay)

(event EventTick
  (params (DeltaSeconds :type Float%20%28single-precision%29)))

(event Input|ActionEvents|InputActionUI_OK
  (params (Key :type Key%20Structure :default "None"))
  (:Pressed
    (bind _asgm_main_menu (Utilities|Casting|CastToGM_MainMenu (Game|GetGameMode)))
    (Default|PressOK _asgm_main_menu)))

(event Input|ActionEvents|InputActionUI_DOWN
  (params (Key :type Key%20Structure :default "None"))
  (:Pressed
    (bind _asgm_main_menu (Utilities|Casting|CastToGM_MainMenu (Game|GetGameMode)))
    (Default|PressDown _asgm_main_menu)))

(event Input|ActionEvents|InputActionUI_UP
  (params (Key :type Key%20Structure :default "None"))
  (:Pressed
    (bind _asgm_main_menu (Utilities|Casting|CastToGM_MainMenu (Game|GetGameMode)))
    (Default|PressUp _asgm_main_menu)))

(event Input|ActionEvents|InputActionUI_Cancel
  (params (Key :type Key%20Structure :default "None"))
  (:Pressed
    (bind _asgm_main_menu (Utilities|Casting|CastToGM_MainMenu (Game|GetGameMode)))
    (Default|PressCancel _asgm_main_menu)))

(fn ConstructionScript)