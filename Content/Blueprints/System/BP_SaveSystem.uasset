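; Save system actor that loads a named save slot, or creates one, and opens its level.
; LoadGame passes an existing save's position to SetMapPosition, which writes it to a separate BP_TempSave slot before the level opens.
; A missing slot gets a new BP_SaveGame with default unit attributes and starting stage, saved before travel.
; SaveGame is a stub that only prints a message.
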(event Custom|SaveGame
  (Development|PrintString "Save Game"))

(event Custom|LoadGame
  (params (SlotName :type String))
  ;[1 1 1] Load
  (bind _returnvalue (SaveGame|DoesSaveGameExist SlotName))
  (if _returnvalue
    (bind _returnvalue_2 (SaveGame|LoadGamefromSlot SlotName))
    (bind _asbp_save_game (Utilities|Casting|CastToBP_SaveGame _returnvalue_2))
    (CallFunction|SetMapPosition (Variables|/Game/Blueprints/System/BP_SaveGame.BP_SaveGame_C|GetPosition _asbp_save_game))
    (Game|OpenLevel(byName) (Utilities|String|StringToName (Variables|/Game/Blueprints/System/BP_SaveGame.BP_SaveGame_C|GetLevelName _asbp_save_game)))
    (else
      (bind _returnvalue_3 (SaveGame|CreateSaveGameObject "/Game/Blueprints/System/BP_SaveGame.BP_SaveGame_C"))
      (bind _asbp_save_game_2 (Utilities|Casting|CastToBP_SaveGame _returnvalue_3))
      (Variables|/Game/Blueprints/System/BP_SaveGame.BP_SaveGame_C|SetUnitAttribute _asbp_save_game_2 (Utilities|Struct|MakeST_UnitAttr 2e+02 1e+01))
      (Variables|/Game/Blueprints/System/BP_SaveGame.BP_SaveGame_C|SetLevelName _asbp_save_game_2 "Stage_0")
      (SaveGame|SaveGametoSlot _asbp_save_game_2 SlotName)
      (Game|OpenLevel(byName) (Utilities|String|StringToName (Variables|/Game/Blueprints/System/BP_SaveGame.BP_SaveGame_C|GetLevelName _asbp_save_game_2))))))

(event Custom|SetMapPosition
  (params (Position :type Vector))
  ;[1 1 1] Load
  (bind _returnvalue (SaveGame|CreateSaveGameObject "/Game/Blueprints/System/BP_TempSave.BP_TempSave_C"))
  (Variables|/Game/Blueprints/System/BP_TempSave.BP_TempSave_C|SetTargetPosition _returnvalue Position)
  (SaveGame|SaveGametoSlot _returnvalue "Temp_Save"))

(event EventBeginPlay)

(event Collision|EventActorBeginOverlap
  (params (OtherActor :type Actor%20Object%20Reference)))

(event EventTick
  (params (DeltaSeconds :type Float%20%28single-precision%29)))

(fn ConstructionScript)