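; Battle game mode that acts as the hub for player UI, interaction focus and battle-control state.
; On BeginPlay it applies any one-shot temp-save position, loads player attributes from save and creates all widgets up front.
; A CurrentUI state routes input to stage selection, NPC talk and weapon switching, toggling visibility and the player state's BattleAble flag.
; Save-point focus is tracked, but its SaveGame call and the interact-hint open/close logic are unwired.
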(event Custom|SetPlayerAttrFromSave
  (bind _asbp_character_base (Utilities|Casting|CastToBP_CharacterBase (Game|GetPlayerCharacter 0)))
  (Default|SetUnitAttrfromSave _asbp_character_base))

(event Custom|OpenUI_InteractHint)

(event Custom|PressUI_Cancel
  (switch string (Variables|Default|GetCurrentUI)
    (:StageSelect
      (Widget|SetVisibility (Variables|Default|GetUI_StageSelect) "Hidden")
      (Widget|SetVisibility (Variables|Default|GetUI_StageSelectHint) "Visible")
      (Variables|Default|SetCurrentUI "StageSelectHint")
      (CallFunction|EnableBattleControl)
      (Variables|Default|SetUI_CurrentFocus 0)
      (bind _asbp_hero_unit (Utilities|Casting|CastToBP_HeroUnit (Game|GetPlayerCharacter 0)))
      (Default|ResetInteractEnable _asbp_hero_unit))))

(event Custom|PressUI_OK
  (bind _ui_stageselect (Variables|Default|GetUI_StageSelect))
  (switch string (Variables|Default|GetCurrentUI)
    (:StageSelect
      (Widget|SetVisibility _ui_stageselect "Hidden")
      (Game|OpenLevel(byName) (Utilities|String|StringToName (Variables|/Game/UI/StageSelect/WBP_StageUnit.WBP_StageUnit_C|GetStageIDName (Variables|/Game/UI/StageSelect/WBP_StageSelect.WBP_StageSelect_C|GetCurrentFocusStage _ui_stageselect))))
      (CallFunction|EnableBattleControl))
    (:NpcPrepareTalk
      (if (Variables|Default|GetisFocusNPC)
        (Default|StartTalk (Variables|Default|GetFocusNPC))
        (CallFunction|DisableBattleControl)
        (Variables|Default|SetCurrentUI "NPCTalk")
        (Widget|SetVisibility (Variables|Default|GetUI_InteractHint) "Hidden")))
    (:NpcTalk
      (Default|EndTalk (Variables|Default|GetFocusNPC))
      (Variables|Default|SetCurrentUI "NPCPrepareTalk")
      (Utilities|FlowControl|Delay 0.1)
      (CallFunction|EnableBattleControl))))

(event Custom|ClearFocusNPC
  (Variables|Default|SetFocusNPC 0)
  (Variables|Default|SetisFocusNPC false)
  (Variables|/Game/Blueprints/BP_MyPlayerState.BP_MyPlayerState_C|SetControlState (Variables|Default|GetMyPlayerState) 0)
  (Variables|Default|SetCurrentUI ""))

(event Custom|OpenUI_SaveHint
  (Widget|SetVisibility (Variables|Default|GetUI_SaveHint) "Visible"))

(event Custom|CloseUI_SaveHint
  (Widget|SetVisibility (Variables|Default|GetUI_SaveHint) "Hidden"))

(event Custom|SetFocusSavePoint
  (params (NewParam :type Save%20Point%20Object%20Reference))
  (Variables|Default|SetFocusSavePoint NewParam)
  (Variables|Default|SetisFocusSavePoint true)
  (Variables|/Game/Blueprints/BP_MyPlayerState.BP_MyPlayerState_C|SetControlState (Variables|Default|GetMyPlayerState) 1)
  (Variables|Default|SetCurrentUI "SaveHint"))

(event Custom|ClearFocusSavePoint
  (Variables|Default|SetFocusSavePoint 0)
  (Variables|Default|SetisFocusSavePoint false)
  (Variables|/Game/Blueprints/BP_MyPlayerState.BP_MyPlayerState_C|SetControlState (Variables|Default|GetMyPlayerState) 0)
  (Variables|Default|SetCurrentUI ""))

(event Custom|DisableBattleControl
  (Variables|/Game/Blueprints/BP_MyPlayerState.BP_MyPlayerState_C|SetBattleAble (Variables|Default|GetMyPlayerState) false))

(event Custom|EnableBattleControl
  (Variables|/Game/Blueprints/BP_MyPlayerState.BP_MyPlayerState_C|SetBattleAble (Variables|Default|GetMyPlayerState) true))

(event Custom|SetFocusStageSelect
  (Variables|Default|SetCurrentUI "StageSelectHint")
  (Widget|SetVisibility (Variables|Default|GetUI_StageSelectHint) "Visible"))

(event Custom|SetupUI
  (Utilities|FlowControl|Sequence
    (:then_0
      (bind _returnvalue (UserInterface|CreateWidget "/Game/UI/StageSelect/WBP_StageSelect.WBP_StageSelect_C"))
      (bind _output_get (Variables|Default|SetUI_StageSelect _returnvalue))
      (Default|SetupUI _output_get)
      (Widget|SetVisibility _output_get "Hidden")
      (UserInterface|Viewport|AddtoViewport _output_get 0))
    (:then_1
      (bind _returnvalue_2 (UserInterface|CreateWidget "/Game/UI/NPC/WBP_InteractHint.WBP_InteractHint_C"))
      (bind _output_get_2 (Variables|Default|SetUI_InteractHint _returnvalue_2))
      (Widget|SetVisibility _output_get_2 "Hidden")
      (UserInterface|Viewport|AddtoViewport _output_get_2 0))
    (:then_2
      (bind _returnvalue_3 (UserInterface|CreateWidget "/Game/UI/NPC/WBP_FullTalk.WBP_FullTalk_C"))
      (bind _output_get_3 (Variables|Default|SetUI_FullTalk _returnvalue_3))
      (Widget|SetVisibility _output_get_3 "Hidden")
      (UserInterface|Viewport|AddtoViewport _output_get_3 0))
    (:then_3
      (bind _returnvalue_4 (UserInterface|CreateWidget "/Game/UI/SavePoint/WBP_SaveHint.WBP_SaveHint_C"))
      (bind _output_get_4 (Variables|Default|SetUI_SaveHint _returnvalue_4))
      (Widget|SetVisibility _output_get_4 "Hidden")
      (UserInterface|Viewport|AddtoViewport _output_get_4 0))
    (:then_4
      (bind _returnvalue_5 (UserInterface|CreateWidget "/Game/UI/StageSelect/WBP_StageSelectHint.WBP_StageSelectHint_C"))
      (bind _output_get_5 (Variables|Default|SetUI_StageSelectHint _returnvalue_5))
      (Widget|SetVisibility _output_get_5 "Hidden")
      (UserInterface|Viewport|AddtoViewport _output_get_5 0))
    (:then_5
      (bind _returnvalue_6 (UserInterface|CreateWidget "/Game/UI/WBP_PlayerHUD.WBP_PlayerHUD_C"))
      (bind _output_get_6 (Variables|Default|SetUI_PlayerHUD _returnvalue_6))
      (Widget|SetVisibility _output_get_6 "Visible")
      (UserInterface|Viewport|AddtoViewport _output_get_6 0))
    (:then_6
      (bind _returnvalue_7 (UserInterface|CreateWidget "/Game/UI/WeaponSelect/WBP_WeaponSelect.WBP_WeaponSelect_C"))
      (bind _output_get_7 (Variables|Default|SetUI_WeaponSelect _returnvalue_7))
      (Default|SetupUI _output_get_7)
      (Widget|SetVisibility _output_get_7 "Hidden")
      (UserInterface|Viewport|AddtoViewport _output_get_7 0))))

(event Custom|ClearFocueStageSelect
  (Variables|Default|SetCurrentUI "")
  (Widget|SetVisibility (Variables|Default|GetUI_StageSelectHint) "Hidden"))

(event Custom|UpdateHPBar
  (params (HP_prcent :type Float%20%28single-precision%29))
  (Progress|SetPercent (Variables|/Game/UI/WBP_PlayerHUD.WBP_PlayerHUD_C|GetHP_Bar (Variables|Default|GetUI_PlayerHUD)) HP_prcent))

(event Custom|OpenStageSelectUI
  (Widget|SetVisibility (Variables|Default|GetUI_StageSelect) "Visible")
  (Widget|SetVisibility (Variables|Default|GetUI_StageSelectHint) "Hidden")
  (Variables|Default|SetCurrentUI "StageSelect")
  (CallFunction|DisableBattleControl)
  (Variables|Default|SetUI_CurrentFocus (Variables|Default|GetUI_StageSelect)))

(event Custom|OpenUI_WeaponSelect
  ;[1 1 1] WeaponSelect
  (Widget|SetVisibility (Variables|Default|GetUI_WeaponSelect) "Visible")
  (Variables|Default|SetCurrentUI "WeaponSelect"))

(event Custom|CloseUI_WeaponSelect
  ;[1 1 1] WeaponSelect
  (Widget|SetVisibility (Variables|Default|GetUI_WeaponSelect) "Hidden")
  (Variables|Default|SetCurrentUI ""))

(event Custom|UI_PressSelectWeapon
  (params (SlotID :type Integer))
  (bind _returnvalue (Game|GetPlayerCharacter 0))
  (bind _asbp_hero_unit (Utilities|Casting|CastToBP_HeroUnit _returnvalue))
  ;[1 1 1] WeaponSelect
  (if (Utilities|Enum|Equal(Enum) (Variables|Default|GetCurrentUI) "WeaponSelect")
    (Default|SetWeaponUI (Variables|Default|GetUI_WeaponSelect) SlotID)
    (Default|SwitchWeapon _asbp_hero_unit (Variables|/Game/UI/WeaponSelect/WBP_WeaponUnit.WBP_WeaponUnit_C|GetWeaponClass (Variables|/Game/UI/WeaponSelect/WBP_WeaponSelect.WBP_WeaponSelect_C|GetCurrentFisrtWeapon (Variables|Default|GetUI_WeaponSelect))) 1)
    (Default|SwitchWeapon _asbp_hero_unit (Variables|/Game/UI/WeaponSelect/WBP_WeaponUnit.WBP_WeaponUnit_C|GetWeaponClass (Variables|/Game/UI/WeaponSelect/WBP_WeaponSelect.WBP_WeaponSelect_C|GetCurrentSecondWeapon (Variables|Default|GetUI_WeaponSelect))) 2)))

(event Custom|UI_WeaponAngle
  (params (Angle :type Float%20%28single-precision%29))
  ;[1 1 1] WeaponSelect
  (Default|WeaponAngleHandle (Variables|Default|GetUI_WeaponSelect) Angle))

(event Custom|OpenStageSelect
  (Widget|SetVisibility (Variables|Default|GetUI_StageSelect) "Visible")
  (Variables|Default|SetCurrentUI "StageSelect")
  (Development|PrintString "Set")
  (Variables|Default|SetUI_CurrentFocus (Variables|Default|GetUI_StageSelect))
  (Development|PrintString "Set"))

(event Custom|PressUI_Up
  (Default|PressUp (Variables|Default|GetUI_CurrentFocus)))

(event Custom|CloseUI_InteractHint)

(event Custom|PressUI_Right
  (Default|PressRight (Variables|Default|GetUI_CurrentFocus)))

(event Custom|PressUI_Down
  (Default|PressDown (Variables|Default|GetUI_CurrentFocus)))

(event Custom|SetFocusNPC
  (params (NPC :type BP%20NPC%20Object%20Reference))
  (Variables|Default|SetFocusNPC NPC)
  (Variables|Default|SetisFocusNPC true)
  (Variables|/Game/Blueprints/BP_MyPlayerState.BP_MyPlayerState_C|SetControlState (Variables|Default|GetMyPlayerState) 1)
  (Variables|Default|SetCurrentUI "NpcPrepareTalk"))

(event Custom|PressUI_Left
  (Default|PressLeft (Variables|Default|GetUI_CurrentFocus)))

(event EventBeginPlay
  (Utilities|FlowControl|Sequence
    (:then_0
      (bind _returnvalue (SaveGame|DoesSaveGameExist "Temp_Save"))
      (if _returnvalue
        (bind _returnvalue_2 (SaveGame|LoadGamefromSlot "Temp_Save"))
        (bind _asbp_temp_save (Utilities|Casting|CastToBP_TempSave _returnvalue_2))
        (Transformation|Teleport (Game|GetPlayerCharacter 0) (Variables|/Game/Blueprints/System/BP_TempSave.BP_TempSave_C|GetTargetPosition _asbp_temp_save) "0, 0, 0")
        (SaveGame|DeleteGameinSlot "Temp_Save")))
    (:then_1
      (CallFunction|SetPlayerAttrfromSave))
    (:then_2
      (CallFunction|SetupUI))
    (:then_3
      (Variables|Default|SetMyPlayerState (.AsBP%20My%20Player%20State (Utilities|Casting|CastToBP_MyPlayerState (Variables|/Script/Engine.Controller|GetPlayerState (.AsBP%20Player%20Controller (Utilities|Casting|CastToBP_PlayerController (Game|GetPlayerController 0))))))))))

(event EventTick
  (params (DeltaSeconds :type Float%20%28single-precision%29)))

(fn ConstructionScript)